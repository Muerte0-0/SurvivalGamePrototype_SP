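; Blueprint function library that exposes the player's default settings and debug flags to other Blueprints.
; GetPlayerDefaultSettings returns the DefaultSettingsData asset as the single source for these values.
; Debug reads its DebugMode flag, and DebugTraces returns TraceDebugMode only while DebugMode is on, otherwise None, so one master switch gates trace drawing.
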(fn GetPlayerDefaultSettings
  (return (LocalVariables|GetDefaultSettingsData)))

(fn Debug
  (return (Variables|/Game/Blueprints/Libraries/Data/PDA_GlobalPlayerSettings.PDA_GlobalPlayerSettings_C|GetDebugMode (Settings|GetPlayerDefaultSettings))))

(fn DebugTraces
  (bind _settings (Settings|GetPlayerDefaultSettings))
  (return (select (Variables|/Game/Blueprints/Libraries/Data/PDA_GlobalPlayerSettings.PDA_GlobalPlayerSettings_C|GetDebugMode _settings) (Variables|/Game/Blueprints/Libraries/Data/PDA_GlobalPlayerSettings.PDA_GlobalPlayerSettings_C|GetTraceDebugMode _settings) "None")))