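; Blueprint function library with a utility that switches a player controller between UI and gameplay input.
; SwitchInputMode takes a UI flag: when true, it sets Game and UI mode focused on the given widget, shows the cursor and moves it to the screen centre.
; When false, it restores Game Only input without flushing and hides the cursor.
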(fn SwitchInputMode
  (params (UI? :type Boolean) (Controller :type Player%20Controller%20Object%20Reference) (WidgetInFocus :type User%20Widget%20Object%20Reference))
  (bind _returnvalue (CallFunction|GetScreenCentre))
  (if UI?
    (Input|SetInputModeGameandUI Controller WidgetInFocus "DoNotLock" false false)
    (Variables|/Script/Engine.PlayerController|SetbShowMouseCursor Controller true)
    (Class|PlayerController|SetMouseLocation Controller (Math|Float|Truncate (.x _returnvalue)) (Math|Float|Truncate (.y _returnvalue)))
    (else
      (Input|SetInputModeGameOnly Controller false)
      (Variables|/Script/Engine.PlayerController|SetbShowMouseCursor Controller false))))