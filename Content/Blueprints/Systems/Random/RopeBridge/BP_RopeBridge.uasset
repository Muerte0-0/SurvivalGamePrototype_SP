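; Procedural rope bridge actor that builds a chain of physics-linked planks in its construction script, sized by Length.
; GeneratePlanks lays static mesh components at even spacing along local Y and stores them in Planks.
; GenerateConstraints adds a rotated physics constraint near the midpoint between each neighbouring pair, joining them.
; Physics simulation is then switched off on the first and last planks, anchoring both ends of the span.
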(fn ConstructionScript
  (CallFunction|GeneratePlanks)
  (CallFunction|GenerateConstraints)
  (Physics|SetSimulatePhysics (Utilities|Array|Get(acopy) (Variables|Default|GetPlanks)) false))

(fn GeneratePlanks
  (Utilities|Array|Clear (Variables|Default|GetPlanks))
  (for _index (range 0 (- (Variables|Default|GetLength) 1))
    (bind _returnvalue (AddComponent|AddStaticMeshComponent false (Math|Transform|MakeTransform (Math|Vector|MakeVector 0.0 (Math|Conversions|ToFloat(Integer) (* _index 65)) 0.0) "0, 0, 0" "1.000000,1.000000,1.000000")))
    (Utilities|Array|Add (Variables|Default|GetPlanks) _returnvalue))
  (return))

(fn GenerateConstraints
  (for _index (range 0 (- (Variables|Default|GetLength) 2))
    (bind _returnvalue (AddComponent|AddPhysicsConstraintComponent false (Math|Transform|MakeTransform (Math|Vector|MakeVector 0.0 (+ (.y (Variables|/Script/Engine.SceneComponent|GetRelativeLocation (Utilities|Array|Get(acopy) (Variables|Default|GetPlanks) _index))) 32.0) 0.0) "0.000000,0.000000,90.000000" "1.000000,1.000000,1.000000")))
    (Class|PhysicsConstraintComponent|SetConstrainedComponents _returnvalue (Utilities|Array|Get(acopy) (Variables|Default|GetPlanks) _index) "None" (Utilities|Array|Get(acopy) (Variables|Default|GetPlanks) (+ _index 1)) "None")))