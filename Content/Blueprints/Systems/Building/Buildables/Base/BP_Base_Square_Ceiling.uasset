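; BP_Base_Square_Ceiling is a square ceiling piece in the building system's buildable base set.
; It exposes nine snap boxes through GetSnapPoints: four for floors, four for walls and one for stairs, presumably so other pieces can attach to it.
; Its construction script only calls the parent's, leaving shared setup to the parent class.
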(fn ConstructionScript
  (|CallParentFunction))

(fn GetSnapPoints
  (return (Utilities|Array|MakeArray (Variables|Default|GetFloorBox1) (Variables|Default|GetFloorBox2) (Variables|Default|GetFloorBox3) (Variables|Default|GetFloorBox4) (Variables|Default|GetWallBox2) (Variables|Default|GetWallBox1) (Variables|Default|GetWallBox3) (Variables|Default|GetWallBox4) (Variables|Default|GetStairsBox))))