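; Base Blueprint for triangle foundation pieces in the building system.
; It overrides GetSnapPoints to return its snap box components, grouped by name for square foundations, walls and triangle foundations.
; The construction script only calls the parent, and the file shows no other logic of its own.
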(fn ConstructionScript
  (|CallParentFunction))

(fn GetSnapPoints
  (return (Utilities|Array|MakeArray (Variables|Default|GetFoundationBox3) (Variables|Default|GetFoundationBox2) (Variables|Default|GetWallBox3) (Variables|Default|GetWallBox2) (Variables|Default|GetWallBox1) (Variables|Default|GetFoundationBox1) (Variables|Default|GetTriFoundationBox1) (Variables|Default|GetTriFoundationBox2) (Variables|Default|GetTriFoundationBox3) (Variables|Default|GetTriFoundationBox5) (Variables|Default|GetTriFoundationBox6) (Variables|Default|GetFoundationBox6) (Variables|Default|GetFoundationBox5) (Variables|Default|GetFoundationBox4) (Variables|Default|GetTriFoundationBox4))))