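; BP_Wood_Foundation is the wooden foundation piece of the building system, a buildable that other pieces can snap onto.
; It overrides GetSnapPoints to return its box components: four for adjacent foundations, four for walls and one for stairs.
; The construction script only calls the parent, and the file holds no other logic.
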(fn ConstructionScript
  (|CallParentFunction))

(fn GetSnapPoints
  (return (Utilities|Array|MakeArray (Variables|Default|GetFoundationBox3) (Variables|Default|GetFoundationBox4) (Variables|Default|GetFoundationBox2) (Variables|Default|GetFoundationBox1) (Variables|Default|GetWallBox2) (Variables|Default|GetWallBox4) (Variables|Default|GetWallBox3) (Variables|Default|GetWallBox1) (Variables|Default|GetStairsBox))))