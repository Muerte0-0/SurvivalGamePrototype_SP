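; BP_Wood_Ceiling is the wooden ceiling piece of the building system.
; It overrides GetSnapPoints to return eight box components, four for floor snapping and four for wall snapping.
; Its construction script only calls the parent's, and its event graph holds only disabled default events, so any other behavior comes from the parent class.
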(event EventBeginPlay)

(event Collision|EventActorBeginOverlap
  (params (OtherActor :type Actor%20Object%20Reference)))

(event EventTick
  (params (DeltaSeconds :type Float%20%28single-precision%29)))

(fn ConstructionScript
  (|CallParentFunction))

(fn GetSnapPoints
  (return (Utilities|Array|MakeArray (Variables|Default|GetFloorBox1) (Variables|Default|GetFloorBox2) (Variables|Default|GetFloorBox3) (Variables|Default|GetFloorBox4) (Variables|Default|GetWallBox2) (Variables|Default|GetWallBox1) (Variables|Default|GetWallBox3) (Variables|Default|GetWallBox4))))