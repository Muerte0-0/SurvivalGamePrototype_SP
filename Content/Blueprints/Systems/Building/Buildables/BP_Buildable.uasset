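; Base Blueprint for placeable building pieces, with snap-point rotation, destruction and empty Repair and Upgrade events.
; Construction sets the mesh from class defaults and shows snap points per a debug-trace setting; GetSnapPoints returns nothing here.
; Tick destroys the piece when its support check overlaps no supporting class.
; Destroy disables visuals and collision, refunds a quarter of resources to any valid player, then swaps in a destructible actor.
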(event EventRotate
  (params (Player :type BP%20Player%20Character%20Object%20Reference))
  (bind _returnvalue (Transformation|GetActorRotation))
  (if (Variables|Default|GetCanRotateAfterPlaced)
    (Transformation|SetActorRotation (Math|Rotator|MakeRotator (.roll _returnvalue) (.pitch _returnvalue) (+ (.yaw _returnvalue) (Variables|Preview|GetRotationSnapAmount))))))

(event EventDestroy
  (params (Player :type BP%20Player%20Character%20Object%20Reference))
  (CallFunction|DisableBuildable)
  (Utilities|IsValid Player
    (:Is%20Valid
      (bind _playerinventory (Variables|/Game/Blueprints/Characters/Player/BP_PlayerCharacter.BP_PlayerCharacter_C|GetPlayerInventory Player)
        (:then
          (for _array_element (Variables|Default|GetResourcesRequired)
            (bind _returnvalue (Game|ConstructObjectfromClass (.Item (Utilities|Struct|BreakS_Item _array_element))))
            (Default|AddItemtoInventory _playerinventory (Utilities|Struct|MakeS_InventoryContent _returnvalue (/ (.Quantity (Utilities|Struct|BreakS_Item _array_element)) 4)))))
        (:else)))
    (:Is%20Not%20Valid
      _))
  (Game|SpawnActorfromClass (Variables|Default|GetDestructibleActor) (Transformation|GetActorTransform) "AdjustIfPossibleButAlwaysSpawn" "MultiplyWithRoot" 0 0)
  (Actor|DestroyActor))

(event EventRepair
  (params (Player :type BP%20Player%20Character%20Object%20Reference)))

(event EventUpgrade
  (params (Player :type BP%20Player%20Character%20Object%20Reference)))

(event EventTick
  (params (DeltaSeconds :type Float%20%28single-precision%29))
  (if (not (CallFunction|HasSupport))
    (CallFunction|Destroy)))

(fn ConstructionScript
  (Components|StaticMesh|SetStaticMesh (Variables|Default|GetBuildingMesh) (Utilities|GetClassDefaults (Variables|Default|GetBuildableObject)))
  (bind _boxes (CallFunction|GetSnapPoints))
  (for _array_element _boxes
    (Development|SetHiddeninGame _array_element (Utilities|Select :Index (CallFunction|DebugTraces) :None true :ForOneFrame false :ForDuration false :Persistent false) false)))

(fn DisableBuildable
  (Rendering|SetVisibility (Variables|Default|GetBuildingMesh) false false)
  (bind _boxes (CallFunction|GetSnapPoints))
  (for _array_element _boxes
    (Collision|SetCollisionEnabled _array_element "NoCollision"))
  (Collision|SetCollisionEnabled (Variables|Default|GetBuildingMesh) "NoCollision"))

(fn HasSupport
  (for _array_element (Variables|Default|GetSupportClasses)
    (if (Utilities|Array|IsNotEmpty (Collision|GetOverlappingActors (Variables|Default|GetSupportCheck) _array_element :!class /Script/Engine.PrimitiveComponent))
      (return true)))
  (return false))

(fn GetSnapPoints
  (return 0))