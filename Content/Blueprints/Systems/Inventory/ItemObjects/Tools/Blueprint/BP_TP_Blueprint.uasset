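; Held blueprint tool item that lets the player pick and place buildables through the player's BuildingComponent.
; Secondary use shows a lazily created, reused WB_BuildPlan radial menu in UI input mode; releasing it hides the menu and restores input.
; Selecting a slot closes the menu and enters build mode with that buildable.
; Primary use spawns the build while the menu is closed, and destroying the tool exits build mode.
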(event Custom|SelectedSlot_Event
  (params (Index :type Integer))
  (CallFunction|HideMenu)
  (bind _player (Variables|Default|GetPlayer)
    (:then
      (bind _buildingcomponent (Variables|/Game/Blueprints/Characters/Player/BP_PlayerCharacter.BP_PlayerCharacter_C|GetBuildingComponent _player)
        (:then
          (Default|EnterBuildMode _buildingcomponent (Utilities|Array|Get(acopy) (Variables|Default|GetBuildables) Index)))
        (:else)))
    (:else)))

(event Custom|HideMenu
  (bind _buildplandmenu (Variables|Default|GetBuildPlandMenu)
    (:then
      (Widget|SetVisibility _buildplandmenu "Hidden")
      (CallFunction|SwitchInputMode false (Game|GetPlayerController 0))
      (Variables|Default|SetInMenu false))
    (:else)))

(event EventDestroyed
  (bind _player (Variables|Default|GetPlayer)
    (:then
      (bind _buildingcomponent (Variables|/Game/Blueprints/Characters/Player/BP_PlayerCharacter.BP_PlayerCharacter_C|GetBuildingComponent _player)
        (:then
          (Default|ExitBuildMode _buildingcomponent))
        (:else)))
    (:else)))

(event EventPrimaryUse
  (if (not (Variables|Default|GetInMenu))
    (Default|SpawnBuild (Variables|/Game/Blueprints/Characters/Player/BP_PlayerCharacter.BP_PlayerCharacter_C|GetBuildingComponent (Variables|Default|GetPlayer)))))

(event EventStopPrimaryUse)

(event EventSecondaryUse
  (bind _buildplandmenu (Variables|Default|GetBuildPlandMenu)
    (:then
      (Widget|SetVisibility _buildplandmenu "Visible"))
    (:else
      (bind _returnvalue (UserInterface|CreateWidget "/Game/Blueprints/Systems/Inventory/ItemObjects/Tools/Blueprint/WB_BuildPlan.WB_BuildPlan_C" 0 (Variables|Default|GetBuildables)))
      (bind _output_get (Variables|Default|SetBuildPlandMenu _returnvalue))
      (UserInterface|Viewport|AddtoViewport _output_get 0)
      (EventDispatchers|AssignSelectedSlot (Variables|/Game/Blueprints/Systems/Inventory/ItemObjects/Tools/Blueprint/WB_BuildPlan.WB_BuildPlan_C|GetWB_RadialWheel _output_get) (delegate Custom|SelectedSlot_Event))))
  (CallFunction|SwitchInputMode true (Game|GetPlayerController 0))
  (Variables|Default|SetInMenu true))

(event EventStopSecondaryUse
  (bind _buildplandmenu (Variables|Default|GetBuildPlandMenu)
    (:then
      (Widget|SetVisibility _buildplandmenu "Hidden")
      (CallFunction|SwitchInputMode false (Game|GetPlayerController 0))
      (Variables|Default|SetInMenu false))
    (:else)))

(fn ConstructionScript
  (|CallParentFunction))