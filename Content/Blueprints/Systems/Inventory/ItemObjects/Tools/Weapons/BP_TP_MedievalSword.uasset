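; Third-person medieval sword item object that performs a melee attack on primary use.
; Primary use, only while not falling, plays a downward attack montage, disables movement and opens a gate until the montage blends out, completes or is interrupted.
; While open, each tick sphere-traces between the mesh's Start and End sockets, applying damage and spending item durability once per continuous contact via a resettable DoOnce.
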(event EventTick
  (params (DeltaSeconds :type Float%20%28single-precision%29))
  (bind _itemmesh (Variables|Default|GetItemMesh))
  (Utilities|FlowControl|Gate true
    (:Exit
      (bind (_outhit _returnvalue) (Collision|SphereTraceByChannel (Transformation|GetSocketLocation _itemmesh "Start") (Transformation|GetSocketLocation _itemmesh "End") 1e+01 "TraceTypeQuery1" false (Utilities|Array|MakeArray (Variables|Default|GetPlayer)) (CallFunction|DebugTraces)))
      (if _returnvalue
        (Utilities|FlowControl|DoOnce false :!label _label
          (:Completed
            (Game|Damage|ApplyDamage (.HitActor (Collision|BreakHitResult _outhit)) 3.0 (Game|GetInstigatorController (Components|GetOwner)) self "/Script/Engine.DamageType")
            (Default|UseDurability (Variables|Default|GetItemObject) 1.0)))
        (else
          (goto _label Reset))))))

(event EventPrimaryUse
  (bind _itemmesh (Variables|Default|GetItemMesh))
  (bind _player (Variables|Default|GetPlayer))
  (bind _player_2 (Variables|Default|GetPlayer))
  (bind _charactermovement (Variables|/Script/Engine.Character|GetCharacterMovement _player))
  (if (not (AI|Components|NavMovement|IsFalling (Variables|/Script/Engine.Character|GetCharacterMovement _player_2)))
    (Animation|Montage|PlayMontage (Variables|/Script/Engine.Character|GetMesh _player_2) "/Game/Assets_Free/Characters/CubeMan/Animations/FullBody/Melee/Standing_Melee_Attack_Downward_Montage.Standing_Melee_Attack_Downward_Montage"
      (:then
        (Pawn|Components|CharacterMovement|DisableMovement _charactermovement)
        (Utilities|FlowControl|Gate true) ; enters at Open
      )
      (:OnCompleted
        (Pawn|Components|CharacterMovement|SetMovementMode _charactermovement "MOVE_Walking" 0 :!label _label)
        (Utilities|FlowControl|Gate true) ; enters at Close
      )
      (:OnBlendOut
        (goto _label))
      (:OnInterrupted
        (goto _label)))))

(fn ConstructionScript
  (|CallParentFunction))