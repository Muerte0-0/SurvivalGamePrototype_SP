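; BP_TP_BuildHammer is a build hammer tool whose secondary use opens a radial menu for upgrading, repairing, destroying or rotating buildables; primary use is empty.
; The menu widget is created once, then shown or hidden while toggling UI input mode.
; Selecting a slot hides the menu and sends the matching message to the actor hit by a short camera trace.
; In third person, the trace start is pushed forward by the spring arm length.
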(event Custom|SelectedSlot_Event
  (params (Index :type Integer))
  (bind _player (Variables|Default|GetPlayer))
  (CallFunction|HideMenu)
  (bind _hitactor (CallFunction|TraceforBuiladable))
  (switch int Index
    (:0
      (Class|BPIBuildable|Upgrade(Message) _hitactor _player))
    (:1
      (Class|BPIBuildable|Repair(Message) _hitactor _player))
    (:2
      (Class|BPIBuildable|Destroy(Message) _hitactor _player))
    (:3
      (Class|BPIBuildable|Rotate(Message) _hitactor _player))))

(event Custom|HideMenu
  (bind _buildhammermenu (Variables|Default|GetBuildHammerMenu)
    (:then
      (Widget|SetVisibility _buildhammermenu "Hidden")
      (CallFunction|SwitchInputMode false (Game|GetPlayerController 0)))
    (:else)))

(event EventPrimaryUse)

(event EventSecondaryUse
  (bind _buildhammermenu (Variables|Default|GetBuildHammerMenu)
    (:then
      (Widget|SetVisibility _buildhammermenu "Visible"))
    (:else
      (bind _returnvalue (UserInterface|CreateWidget "/Game/Blueprints/Systems/Inventory/ItemObjects/Tools/BuildHammer/WB_BuildHammerMenu.WB_BuildHammerMenu_C"))
      (bind _output_get (Variables|Default|SetBuildHammerMenu _returnvalue))
      (UserInterface|Viewport|AddtoViewport _output_get 0)
      (EventDispatchers|AssignSelectedSlot (Variables|/Game/Blueprints/Systems/Inventory/ItemObjects/Tools/BuildHammer/WB_BuildHammerMenu.WB_BuildHammerMenu_C|GetWB_RadialWheel _output_get) (delegate Custom|SelectedSlot_Event))))
  (CallFunction|SwitchInputMode true (Game|GetPlayerController 0) (Variables|Default|GetBuildHammerMenu)))

(event EventStopSecondaryUse
  (bind _buildhammermenu (Variables|Default|GetBuildHammerMenu)
    (:then
      (Widget|SetVisibility _buildhammermenu "Hidden")
      (CallFunction|SwitchInputMode false (Game|GetPlayerController 0)))
    (:else)))

(fn ConstructionScript
  (|CallParentFunction))

(fn TraceforBuiladable
  (bind (_start _end) (CallFunction|GetTraceStartEnd 5e+02))
  (bind (_outhit _returnvalue) (Collision|LineTraceByChannel _start _end "TraceTypeQuery1" false (Utilities|Array|MakeArray (Components|GetOwner)) (CallFunction|DebugTraces)))
  (if _returnvalue
    (return (.HitActor (Collision|BreakHitResult _outhit)))
    (else
      (return 0))))

(fn GetTraceStartEnd
  (params (Range :type Float%20%28single-precision%29))
  (bind _player (Variables|Default|GetPlayer))
  (bind (_cameracomponent _fpp_) (Default|GetCamera _player))
  (bind _returnvalue (Transformation|GetWorldLocation _cameracomponent))
  (bind _returnvalue_2 (Math|Vector|GetForwardVector _cameracomponent))
  (return (+ _returnvalue (* _returnvalue_2 (Math|Float|SelectFloat 1.0 (Variables|/Script/Engine.SpringArmComponent|GetTargetArmLength (Variables|/Game/Blueprints/Characters/Player/BP_PlayerCharacter.BP_PlayerCharacter_C|GetSpringArm _player)) _fpp_))) (+ _returnvalue (* _returnvalue_2 Range))))