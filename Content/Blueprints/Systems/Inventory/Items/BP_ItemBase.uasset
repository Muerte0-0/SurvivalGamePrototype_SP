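; BP_ItemBase is the base Blueprint for inventory items owned by the player character.
; Its construction script sets the item's skeletal mesh from its ItemObject when that object is valid.
; On BeginPlay it casts its owner to BP_PlayerCharacter and binds to that character's SwitchedPerspective dispatcher.
; Perspective switches pass the FPP value to ToggleVisibility, which is empty here.
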(event Custom|SwitchedPerspective_Event
  (params (FPP? :type Boolean))
  (CallFunction|ToggleVisibility FPP?))

(event EventBeginPlay
  (bind _asbp_player_character (Utilities|Casting|CastToBP_PlayerCharacter (Components|GetOwner)))
  (bind _output_get (Variables|Default|SetPlayer _asbp_player_character))
  (EventDispatchers|AssignSwitchedPerspective _output_get (delegate Custom|SwitchedPerspective_Event)))

(fn ConstructionScript
  (bind _itemobject (Variables|Default|GetItemObject)
    (:then
      (Components|SkeletalMesh|SetSkeletalMeshAsset (Variables|Default|GetItemMesh) (Variables|/Game/Blueprints/Systems/Inventory/Data/ItemObject.ItemObject_C|GetSkeletalMesh _itemobject)))
    (:else)))

(fn ToggleVisibility
  (params (FPP? :type Boolean)))