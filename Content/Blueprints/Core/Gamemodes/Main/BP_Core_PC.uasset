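; BP_Core_PC is the core player controller that owns the player's HUD and toggles its inventory view.
; CreateHUD builds a WB_PlayerHUD widget from the supplied inventory and equipment component, stores it and adds it to the viewport.
; ToggleInventory uses the InventoryShown flag to tell that widget to show or hide the inventory, then flips the flag.
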(event Custom|CreateHUD
  (params (PlayerInventory :type Item%20Container%20Component%20Object%20Reference) (EquipmentComponent :type Equipment%20Component%20Object%20Reference))
  (bind _returnvalue (UserInterface|CreateWidget "/Game/Blueprints/Widgets/WB_PlayerHUD.WB_PlayerHUD_C" 0 PlayerInventory EquipmentComponent))
  (bind _output_get (Variables|Default|SetPlayerHUD _returnvalue))
  (UserInterface|Viewport|AddtoViewport _output_get 0))

(event Custom|ToggleInventory
  (if (Variables|Default|GetInventoryShown)
    (Default|HideInventory (Variables|Default|GetPlayerHUD))
    (Variables|Default|SetInventoryShown false)
    (else
      (Default|ShowInventory (Variables|Default|GetPlayerHUD))
      (Variables|Default|SetInventoryShown true))))

(fn ConstructionScript)